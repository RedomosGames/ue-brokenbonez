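; Player character for a ramp trick game where number-key combos typed mid-air earn points.
; Entering a ramp launches the player, shows a random combo, plays a random timeline-driven mesh spin and accrues pending score.
; Landing compares both combo arrays, banking the score or costing a life, and fires GameMode's game over at zero lives.
; GameInstance settings tune play, while pausable looping timers drive score ticks and post-landing repositioning.
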(event Custom|CE_StartTasks
  ;[1 0.783 0 0.5] Start Tasks
  (Utilities|FlowControl|Sequence
    (:then_0
      (bind _returnvalue (Actor|GetActorOfClass "/Game/Blueprints/Gameplay/BP_CameraPos.BP_CameraPos_C"))
      (Transformation|AttachComponentToComponent (Variables|Default|GetCamera) (Variables|/Game/Blueprints/Gameplay/BP_CameraPos.BP_CameraPos_C|GetArrow _returnvalue) "None" "KeepRelative" "KeepRelative" "KeepRelative" true))
    (:then_1
      (CallFunction|CEMovePlayer)
      (CallFunction|CEIncreaseScore))
    (:then_2
      (CallFunction|CESetInitalPlayerValues)
      (CallFunction|CESetInitalUI))
    (:then_3
      (CallFunction|CESetGameSpeed)
      (CallFunction|CEwhenGameOver)
      (CallFunction|CEUpdateTimer))))

(event Custom|CE_LaunchPlayer
  ;[1 0.783 0 0.5] CE_LaunchPlayer - Launch Player into air
  (Character|LaunchCharacter (Math|Vector|MakeVector (Variables|PlayerStats|GetLaunchVelocityX) 0.0 (Variables|PlayerStats|GetLaunchVelocityZ)) false true)
  (Variables|Widget|SetProgressDecreasTime (Variables|Widget|GetProgressDecreasMaxTime)))

(event Custom|CE_CheckComboResult
  ;[1 0.783 0 0.5] CE_CheckComboResult - Check Array Values, Set Landed value
  (if (Utilities|Array|Identical (Variables|TrickCombo|GetTrickCombo) (Variables|TrickCombo|GetPlayerCombo))
    (Variables|PlayerStats|SetPlayerStats (Utilities|Struct|MakeS_PlayerStats (.playerscore (Variables|PlayerStats|GetPlayerStats)) (.scoretoadd (Variables|PlayerStats|GetPlayerStats)) (.playerlives (Variables|PlayerStats|GetPlayerStats)) true))
    (else
      (Variables|PlayerStats|SetPlayerStats (Utilities|Struct|MakeS_PlayerStats (.playerscore (Variables|PlayerStats|GetPlayerStats)) (.scoretoadd (Variables|PlayerStats|GetPlayerStats)) (.playerlives (Variables|PlayerStats|GetPlayerStats)) false))))
  (CallFunction|CEClearAllCombos))

(event Custom|CE_CheckGameOver
  ;[1 0.783 0 0.5] CE_CheckGameOver - check player lives
  (if (> (.PlayerLives (Utilities|Struct|BreakS_PlayerStats (Variables|PlayerStats|GetPlayerStats))) 0)
    (Development|PrintString "Still Alive")
    (else
      (Development|PrintString "Game Over")
      (Default|CallOnGameOver (Variables|Default|GetGmRef)))))

(event Custom|CE_SetInitalPlayerValues
  ;[1 0.783 0 0.5] CE_SetInitalPlayerValues
  ;;[1 0.783 0 0.5] Comment
  (Variables|PlayerStats|SetPlayerStats (Utilities|Struct|MakeS_PlayerStats 0 0 (Utilities|Struct|BreakS_SetGameSettings (Variables|/Game/Blueprints/GI_BrokenBonez.GI_BrokenBonez_C|GetSetGameSettings (Variables|Default|GetGiRef))) false)))

(event Custom|CE_SetInitalUI
  ;[1 0.783 0 0.5] CE_Set Inital UI
  (Utilities|FlowControl|Sequence
    (:then_0
      (bind _returnvalue (UserInterface|CreateWidget "/Game/Blueprints/UI/Gameplay/WBP_PlayerDisplay.WBP_PlayerDisplay_C" (Game|GetPlayerController 0)))
      (bind _output_get (Variables|Widget|SetPlayerDisplayWidgetRef _returnvalue))
      (Variables|Widget|SetScreenInfoWidgetRef (Variables|/Game/Blueprints/UI/Gameplay/WBP_PlayerDisplay.WBP_PlayerDisplay_C|GetWBP_ScreenInfo _output_get))
      (UserInterface|Viewport|AddtoViewport _output_get 0)
      (Variables|Widget|SetGameOverInfoRef (Variables|/Game/Blueprints/UI/Gameplay/WBP_PlayerDisplay.WBP_PlayerDisplay_C|GetWBP_GameOverInfo _output_get)))
    (:then_1
      (CallFunction|CEUpdatePlayerUI))))

(event Custom|CE_SetScoreVisibility
  (params (IsAddedScoreVisible? :type Boolean))
  (bind _screeninfowidgetref (Variables|Widget|GetScreenInfoWidgetRef))
  (bind _txt_addscore (Variables|/Game/Blueprints/UI/Gameplay/WBP_ScreenInfo.WBP_ScreenInfo_C|GetTXT_AddScore _screeninfowidgetref))
  ;[1 0.783 0 0.5] CE_SetAddedScoreVisibility - Hide and show added score text
  (if IsAddedScoreVisible?
    (Widget|SetVisibility _txt_addscore "Visible")
    (else
      (Widget|SetVisibility _txt_addscore "Collapsed"))))

(event Custom|CE_UpdatePlayerUI
  (bind _screeninfowidgetref (Variables|Widget|GetScreenInfoWidgetRef))
  (bind _playerstats (Variables|PlayerStats|GetPlayerStats))
  (bind (_playerscore _playerlives) (Utilities|Struct|BreakS_PlayerStats _playerstats))
  ;[1 0.783 0 0.5] CE_UpdatePlayerUI - Set Score and Lives Text
  (Rendering|Components|TextRender|SetText (Variables|/Game/Blueprints/UI/Gameplay/WBP_ScreenInfo.WBP_ScreenInfo_C|GetTXT_PlayerLives _screeninfowidgetref) (Utilities|Text|FormatText "Player Lives: {Lives}" _playerlives))
  (Rendering|Components|TextRender|SetText (Variables|/Game/Blueprints/UI/Gameplay/WBP_ScreenInfo.WBP_ScreenInfo_C|GetTXT_PlayerScore _screeninfowidgetref) (Utilities|Text|FormatText "Player Score: {Score}" _playerscore))
  (Rendering|Components|TextRender|SetText (Variables|/Game/Blueprints/UI/Gameplay/WBP_ScreenInfo.WBP_ScreenInfo_C|GetTXT_GameTimeLeft _screeninfowidgetref) (Utilities|Text|FormatText "Time Left: 
{TimeLeft}" (Variables|/Game/Blueprints/GM_Gameplay.GM_Gameplay_C|GetGameTimerLeft (Variables|Default|GetGmRef)))))

(event Custom|CE_SetBarTimeLeft
  ;[1 0.783 0 0.5] CE_SetBarTimeLeft - Change the progress bar for time left
  (bind _output_get (Variables|Widget|SetProgressDecreasTime (- (Variables|Widget|GetProgressDecreasTime) 1.0)))
  (Progress|SetPercent (Variables|/Game/Blueprints/UI/Gameplay/WBP_ScreenInfo.WBP_ScreenInfo_C|GetPB_TimeLeftToInoput (Variables|Widget|GetScreenInfoWidgetRef)) (/ _output_get (Variables|Widget|GetProgressDecreasMaxTime))))

(event Custom|CE_SelectComboAnim
  ;[1 0.783 0 0.5] CE_SelectComboAnim - Select Combo Anim
  (CallFunction|FSetEnumOfRanomInt (Math|Random|RandomIntegerinRange 1 6))
  (|SelectAnimTimeline))

(event Custom|CE_SetGameSpeed
  ;[1 0.783 0 0.5] CE_SetGameSpeed
  ;;[1 0.783 0 0.5] Comment
  (Utilities|Time|SetGlobalTimeDilation (Utilities|Struct|BreakS_SetGameSettings (Variables|/Game/Blueprints/GI_BrokenBonez.GI_BrokenBonez_C|GetSetGameSettings (Variables|Default|GetGiRef)))))

(event Custom|CE_WhenGameOver
  ;[1 0.783 0 0.5] CE_WhenGameOver
  (EventDispatchers|BindEventtoOnGameOver (Variables|Default|GetGmRef) (delegate Custom|WhenGameOver)))

(event Custom|CE_MovePlayer
  ;[1 0.783 0 0.5] CE_MovePlayer - Move player back to starting position
  (bind _returnvalue (Utilities|Time|SetTimerbyEvent (delegate Custom|MovePlayer) 0.001 true))
  (bind _output_get (Variables|TimerHandles|SetMovePlayerTimerHandle _returnvalue))
  (Utilities|Time|PauseTimerbyHandle _output_get))

(event Custom|WhenGameOver
  (bind _returnvalue (Game|GetPlayerController 0))
  (bind _playerdisplaywidgetref (Variables|Widget|GetPlayerDisplayWidgetRef))
  (bind _wbp_gameoverinfo (Variables|/Game/Blueprints/UI/Gameplay/WBP_PlayerDisplay.WBP_PlayerDisplay_C|GetWBP_GameOverInfo _playerdisplaywidgetref))
  ;[1 0.783 0 0.5] CE_WhenGameOver
  (Variables|/Script/Engine.SkeletalMeshComponent|SetSkeletalMeshAsset (Variables|Character|GetMesh) 0)
  (Niagara|SpawnSystematLocation "/Niagara/DefaultAssets/Templates/Systems/SimpleExplosion.SimpleExplosion" (Transformation|GetActorLocation))
  (Variables|/Script/Engine.PlayerController|SetbShowMouseCursor _returnvalue true)
  (Input|SetInputModeUIOnly _returnvalue 0 "DoNotLock" false)
  (Utilities|FlowControl|Delay 1.5)
  (Widget|SetVisibility (Variables|/Game/Blueprints/UI/Gameplay/WBP_PlayerDisplay.WBP_PlayerDisplay_C|GetWBP_ScreenInfo _playerdisplaywidgetref) "Collapsed")
  (Widget|SetVisibility _wbp_gameoverinfo "Visible")
  (Rendering|Components|TextRender|SetText (Variables|/Game/Blueprints/UI/Gameplay/WBP_GameOverInfo.WBP_GameOverInfo_C|GetTXT_playerScore _wbp_gameoverinfo) (Utilities|Text|FormatText "Player Score: 
{Score}" (Utilities|Struct|BreakS_PlayerStats (Variables|PlayerStats|GetPlayerStats))))
  (Utilities|Time|SetGlobalTimeDilation 0.0))

(event Custom|CE_UpdateTimer
  ;[1 0.783 0 0.5] CE_UpdateTimer
  (Utilities|Time|SetTimerbyEvent (delegate Custom|UpdateTimer) 0.25 true))

(event Custom|UpdateTimer
  ;[1 0.783 0 0.5] CE_UpdateTimer
  (CallFunction|CEUpdatePlayerUI))

(event Custom|MovePlayer
  (bind _capsulecomponent (Variables|Collision|GetCapsuleComponent))
  (bind _relativelocation (Variables|/Script/Engine.SceneComponent|GetRelativeLocation _capsulecomponent))
  ;[1 0.783 0 0.5] CE_MovePlayer - Move player back to starting position
  (if (> (.x (Variables|/Script/Engine.SceneComponent|GetRelativeLocation (Variables|Collision|GetCapsuleComponent))) -7.5e+02)
    (Transformation|SetRelativeLocation _capsulecomponent (Math|Vector|MakeVector (- (.x _relativelocation) 1.0) (.y _relativelocation) (.z _relativelocation)) false false)
    (else
      (Utilities|Time|PauseTimerbyHandle (Variables|TimerHandles|GetMovePlayerTimerHandle)))))

(event Custom|CE_IncreaseScore
  ;[1 0.783 0 0.5] CE_IncreaseScore - Increase Added score until landing
  (bind _returnvalue (Utilities|Time|SetTimerbyEvent (delegate Custom|IncreaseScore) 0.001 true))
  (bind _output_get (Variables|TimerHandles|SetIncreaseScoreTimerHandle _returnvalue))
  (Utilities|Time|PauseTimerbyHandle _output_get))

(event Custom|IncreaseScore
  ;[1 0.783 0 0.5] CE_IncreaseScore - Increase Added score until landing
  (bind _output_get (Variables|PlayerStats|SetPlayerStats (Utilities|Struct|MakeS_PlayerStats (.PlayerScore (Utilities|Struct|BreakS_PlayerStats (Variables|PlayerStats|GetPlayerStats))) (+ (Utilities|Struct|BreakS_SetGameSettings (Variables|/Game/Blueprints/GI_BrokenBonez.GI_BrokenBonez_C|GetSetGameSettings (Variables|Default|GetGiRef))) (.ScoreToAdd (Utilities|Struct|BreakS_PlayerStats (Variables|PlayerStats|GetPlayerStats)))) (.PlayerLives (Utilities|Struct|BreakS_PlayerStats (Variables|PlayerStats|GetPlayerStats))) (.LandedSuccessfully? (Utilities|Struct|BreakS_PlayerStats (Variables|PlayerStats|GetPlayerStats))))))
  (Rendering|Components|TextRender|SetText (Variables|/Game/Blueprints/UI/Gameplay/WBP_ScreenInfo.WBP_ScreenInfo_C|GetTXT_AddScore (Variables|Widget|GetScreenInfoWidgetRef)) (Utilities|Text|FormatText "{ScoreToAdd}" (Utilities|Struct|BreakS_PlayerStats _output_get)))
  (CallFunction|CESetBarTimeLeft))

(event Custom|CE_AddScore
  ;[1 0.783 0 0.5] CE_AddScore - Check Landed value, if true, add score to player score
  (if (.LandedSuccessfully? (Utilities|Struct|BreakS_PlayerStats (Variables|PlayerStats|GetPlayerStats)))
    (Variables|PlayerStats|SetPlayerStats (Utilities|Struct|MakeS_PlayerStats (+ (.PlayerScore (Utilities|Struct|BreakS_PlayerStats (Variables|PlayerStats|GetPlayerStats))) (.ScoreToAdd (Utilities|Struct|BreakS_PlayerStats (Variables|PlayerStats|GetPlayerStats)))) 0 (.PlayerLives (Utilities|Struct|BreakS_PlayerStats (Variables|PlayerStats|GetPlayerStats))) false))
    (else
      (Variables|PlayerStats|SetPlayerStats (Utilities|Struct|MakeS_PlayerStats (.PlayerScore (Utilities|Struct|BreakS_PlayerStats (Variables|PlayerStats|GetPlayerStats))) 0 (- (.PlayerLives (Utilities|Struct|BreakS_PlayerStats (Variables|PlayerStats|GetPlayerStats))) 1) false))))
  (CallFunction|CEUpdatePlayerUI)
  (CallFunction|CECheckGameOver))

(event Custom|CE_ClearAllCombos
  (bind _screeninfowidgetref (Variables|Widget|GetScreenInfoWidgetRef))
  ;[1 0.783 0 0.5] CE_ClearAllCombos - Clear Both Player Input an Random Input
  (Widget|Panel|ClearChildren (Variables|/Game/Blueprints/UI/Gameplay/WBP_ScreenInfo.WBP_ScreenInfo_C|GetHB_ComboInputDisplay _screeninfowidgetref))
  (Widget|Panel|ClearChildren (Variables|/Game/Blueprints/UI/Gameplay/WBP_ScreenInfo.WBP_ScreenInfo_C|GetHB_PlayerInputDisplay _screeninfowidgetref))
  (Utilities|Array|Clear (Variables|TrickCombo|GetPlayerCombo))
  (Utilities|Array|Clear (Variables|TrickCombo|GetTrickCombo)))

(event Custom|CE_CreateTrickCombo
  (bind _giref (Variables|Default|GetGiRef))
  (bind _setgamesettings (Variables|/Game/Blueprints/GI_BrokenBonez.GI_BrokenBonez_C|GetSetGameSettings _giref))
  (bind (_assignsetcomboamount _assignkeycombokeymax) (Utilities|Struct|BreakS_SetGameSettings _setgamesettings))
  ;[1 0.783 0 0.5] CE_CreateTrickCombo - Select which keys need to be pressed
  ;;[1 0.783 0 0.5] Comment
  (for _index (range 1 _assignsetcomboamount)
    (Utilities|Array|Add (Variables|TrickCombo|GetTrickCombo) (Math|Random|RandomIntegerinRange 1 _assignkeycombokeymax)))
  (for _array_element (Variables|TrickCombo|GetTrickCombo)
    (CallFunction|FSelectRandomIntInputWidget _array_element)))

(event Custom|CE_SetPlayerInputBoxVisibility
  (params (IsPlayerBoxVisisble? :type Boolean))
  (bind _screeninfowidgetref (Variables|Widget|GetScreenInfoWidgetRef))
  (bind _hb_playerinputdisplay (Variables|/Game/Blueprints/UI/Gameplay/WBP_ScreenInfo.WBP_ScreenInfo_C|GetHB_PlayerInputDisplay _screeninfowidgetref))
  (bind _pb_timelefttoinoput (Variables|/Game/Blueprints/UI/Gameplay/WBP_ScreenInfo.WBP_ScreenInfo_C|GetPB_TimeLeftToInoput _screeninfowidgetref))
  ;[1 0.783 0 0.5] CE_SetPlayerInputBoxVisibility - Hide and Show Player Input Box
  (if IsPlayerBoxVisisble?
    (Widget|SetVisibility _hb_playerinputdisplay "Visible")
    (Widget|SetVisibility _pb_timelefttoinoput "Visible")
    (else
      (Widget|SetVisibility _hb_playerinputdisplay "Collapsed")
      (Widget|SetVisibility _pb_timelefttoinoput "Collapsed"))))

(event EventBeginPlay
  ;[1 0.783 0 0.5] Begin Play
  (Utilities|FlowControl|DelayUntilNextTick)
  (bind _asgi_broken_bonez (Utilities|Casting|CastToGI_BrokenBonez (Game|GetGameInstance)))
  (Variables|Default|SetGiRef _asgi_broken_bonez)
  (bind _asgm_gameplay (Utilities|Casting|CastToGM_Gameplay (Game|GetGameMode)))
  (Variables|Default|SetGmRef _asgm_gameplay)
  (CallFunction|CEStartTasks))

(event EventIFLanded
  ;[1 0.783 0 0.5] IF_Landed
  (Utilities|Time|UnpauseTimerbyHandle (Variables|TimerHandles|GetMovePlayerTimerHandle))
  (Utilities|Time|PauseTimerbyHandle (Variables|TimerHandles|GetIncreaseScoreTimerHandle))
  (CallFunction|CECheckComboResult)
  (CallFunction|CEAddScore)
  (CallFunction|CESetScoreVisibility false)
  (CallFunction|CESetPlayerInputBoxVisibility false))

(event EventIFEnterRamp
  ;[1 0.783 0 0.5] IF_EnterRamp
  (CallFunction|CELaunchPlayer)
  (Utilities|Time|UnpauseTimerbyHandle (Variables|TimerHandles|GetIncreaseScoreTimerHandle))
  (CallFunction|CECreateTrickCombo)
  (CallFunction|CESetScoreVisibility true)
  (CallFunction|FClearPlayerInput&Box)
  (CallFunction|CESetPlayerInputBoxVisibility true)
  (CallFunction|CESelectComboAnim))

(event Input|KeyboardEvents|9
  (params (Key :type Key%20Structure :default "None"))
  (bind _9 (Variables|PlayerInputs|Get9))
  ;[1 0.783 0 0.5] Player Input Keys
  (:Pressed
    (Utilities|Array|Add (Variables|TrickCombo|GetPlayerCombo) _9)
    (CallFunction|FSelectPlayerIntInputBox _9)))

(event Input|KeyboardEvents|3
  (params (Key :type Key%20Structure :default "None"))
  (bind _3 (Variables|PlayerInputs|Get3))
  ;[1 0.783 0 0.5] Player Input Keys
  (:Pressed
    (Utilities|Array|Add (Variables|TrickCombo|GetPlayerCombo) _3)
    (CallFunction|FSelectPlayerIntInputBox _3)))

(event Input|KeyboardEvents|4
  (params (Key :type Key%20Structure :default "None"))
  (bind _4 (Variables|PlayerInputs|Get4))
  ;[1 0.783 0 0.5] Player Input Keys
  (:Pressed
    (Utilities|Array|Add (Variables|TrickCombo|GetPlayerCombo) _4)
    (CallFunction|FSelectPlayerIntInputBox _4)))

(event Input|KeyboardEvents|2
  (params (Key :type Key%20Structure :default "None"))
  (bind _2 (Variables|PlayerInputs|Get2))
  ;[1 0.783 0 0.5] Player Input Keys
  (:Pressed
    (Utilities|Array|Add (Variables|TrickCombo|GetPlayerCombo) _2)
    (CallFunction|FSelectPlayerIntInputBox _2)))

(event Input|KeyboardEvents|1
  (params (Key :type Key%20Structure :default "None"))
  (bind _1 (Variables|PlayerInputs|Get1))
  ;[1 0.783 0 0.5] Player Input Keys
  (:Pressed
    (Utilities|Array|Add (Variables|TrickCombo|GetPlayerCombo) _1)
    (CallFunction|FSelectPlayerIntInputBox _1)))

(event Input|KeyboardEvents|5
  (params (Key :type Key%20Structure :default "None"))
  (bind _5 (Variables|PlayerInputs|Get5))
  ;[1 0.783 0 0.5] Player Input Keys
  (:Pressed
    (Utilities|Array|Add (Variables|TrickCombo|GetPlayerCombo) _5)
    (CallFunction|FSelectPlayerIntInputBox _5)))

(event Input|KeyboardEvents|6
  (params (Key :type Key%20Structure :default "None"))
  (bind _6 (Variables|PlayerInputs|Get6))
  ;[1 0.783 0 0.5] Player Input Keys
  (:Pressed
    (Utilities|Array|Add (Variables|TrickCombo|GetPlayerCombo) _6)
    (CallFunction|FSelectPlayerIntInputBox _6)))

(event Input|KeyboardEvents|7
  (params (Key :type Key%20Structure :default "None"))
  (bind _7 (Variables|PlayerInputs|Get7))
  ;[1 0.783 0 0.5] Player Input Keys
  (:Pressed
    (Utilities|Array|Add (Variables|TrickCombo|GetPlayerCombo) _7)
    (CallFunction|FSelectPlayerIntInputBox _7)))

(event Input|KeyboardEvents|8
  (params (Key :type Key%20Structure :default "None"))
  (bind _8 (Variables|PlayerInputs|Get8))
  ;[1 0.783 0 0.5] Player Input Keys
  (:Pressed
    (Utilities|Array|Add (Variables|TrickCombo|GetPlayerCombo) _8)
    (CallFunction|FSelectPlayerIntInputBox _8)))

(fn ConstructionScript)

(fn FAddWidgettoInputBox
  (params (Content :type Widget%20Object%20Reference))
  (Class|HorizontalBox|AddChildtoHorizontalBox (Variables|/Game/Blueprints/UI/Gameplay/WBP_ScreenInfo.WBP_ScreenInfo_C|GetHB_ComboInputDisplay (Variables|Widget|GetScreenInfoWidgetRef)) Content))

(fn FSelectRandomIntInputWidget
  (params (RandomNumberArray :type Integer))
  (Utilities|MCheckNumber RandomNumberArray (Variables|PlayerInputs|Get1)
    (:True
      (bind _returnvalue (UserInterface|CreateWidget "/Game/Blueprints/UI/Gameplay/InputUI/WBP_Input_1.WBP_Input_1_C" (Game|GetPlayerController 0)))
      (CallFunction|FAddWidgettoInputBox _returnvalue))
    (:False
      (Utilities|MCheckNumber RandomNumberArray (Variables|PlayerInputs|Get2)
        (:True
          (bind _returnvalue_2 (UserInterface|CreateWidget "/Game/Blueprints/UI/Gameplay/InputUI/WBP_Input_2.WBP_Input_2_C" (Game|GetPlayerController 0)))
          (CallFunction|FAddWidgettoInputBox _returnvalue_2))
        (:False
          (Utilities|MCheckNumber RandomNumberArray (Variables|PlayerInputs|Get3)
            (:True
              (bind _returnvalue_3 (UserInterface|CreateWidget "/Game/Blueprints/UI/Gameplay/InputUI/WBP_Input_3.WBP_Input_3_C" (Game|GetPlayerController 0)))
              (CallFunction|FAddWidgettoInputBox _returnvalue_3))
            (:False
              (Utilities|MCheckNumber RandomNumberArray (Variables|PlayerInputs|Get4)
                (:True
                  (bind _returnvalue_4 (UserInterface|CreateWidget "/Game/Blueprints/UI/Gameplay/InputUI/WBP_Input_4.WBP_Input_4_C" (Game|GetPlayerController 0)))
                  (CallFunction|FAddWidgettoInputBox _returnvalue_4))
                (:False
                  (Utilities|MCheckNumber 0 (Variables|PlayerInputs|Get5)
                    (:True
                      (bind _returnvalue_5 (UserInterface|CreateWidget "/Game/Blueprints/UI/Gameplay/InputUI/WBP_Input_5.WBP_Input_5_C" (Game|GetPlayerController 0)))
                      (CallFunction|FAddWidgettoInputBox _returnvalue_5))
                    (:False
                      (Utilities|MCheckNumber RandomNumberArray (Variables|PlayerInputs|Get6)
                        (:True
                          (bind _returnvalue_6 (UserInterface|CreateWidget "/Game/Blueprints/UI/Gameplay/InputUI/WBP_Input_6.WBP_Input_6_C" (Game|GetPlayerController 0)))
                          (CallFunction|FAddWidgettoInputBox _returnvalue_6))
                        (:False
                          (Utilities|MCheckNumber RandomNumberArray (Variables|PlayerInputs|Get7)
                            (:True
                              (bind _returnvalue_7 (UserInterface|CreateWidget "/Game/Blueprints/UI/Gameplay/InputUI/WBP_Input_7.WBP_Input_7_C" (Game|GetPlayerController 0)))
                              (CallFunction|FAddWidgettoInputBox _returnvalue_7))
                            (:False
                              (Utilities|MCheckNumber RandomNumberArray (Variables|PlayerInputs|Get8)
                                (:True
                                  (bind _returnvalue_8 (UserInterface|CreateWidget "/Game/Blueprints/UI/Gameplay/InputUI/WBP_Input_8.WBP_Input_8_C" (Game|GetPlayerController 0)))
                                  (CallFunction|FAddWidgettoInputBox _returnvalue_8))
                                (:False
                                  (Utilities|MCheckNumber RandomNumberArray (Variables|PlayerInputs|Get9)
                                    (:True
                                      (bind _returnvalue_9 (UserInterface|CreateWidget "/Game/Blueprints/UI/Gameplay/InputUI/WBP_Input_9.WBP_Input_9_C" (Game|GetPlayerController 0)))
                                      (CallFunction|FAddWidgettoInputBox _returnvalue_9))))))))))))))))))))

(fn FAddWidgettoPlayerBox
  (params (Content :type Widget%20Object%20Reference))
  (Class|HorizontalBox|AddChildtoHorizontalBox (Variables|/Game/Blueprints/UI/Gameplay/WBP_ScreenInfo.WBP_ScreenInfo_C|GetHB_PlayerInputDisplay (Variables|Widget|GetScreenInfoWidgetRef)) Content))

(fn FSelectPlayerIntInputBox
  (params (Player%20Input :type Integer))
  (Utilities|MCheckNumber Player%20Input (Variables|PlayerInputs|Get1)
    (:True
      (bind _returnvalue (UserInterface|CreateWidget "/Game/Blueprints/UI/Gameplay/InputUI/WBP_Input_1.WBP_Input_1_C" (Game|GetPlayerController 0)))
      (CallFunction|FAddWidgettoPlayerBox _returnvalue))
    (:False
      (Utilities|MCheckNumber Player%20Input (Variables|PlayerInputs|Get2)
        (:True
          (bind _returnvalue_2 (UserInterface|CreateWidget "/Game/Blueprints/UI/Gameplay/InputUI/WBP_Input_2.WBP_Input_2_C" (Game|GetPlayerController 0)))
          (CallFunction|FAddWidgettoPlayerBox _returnvalue_2))
        (:False
          (Utilities|MCheckNumber Player%20Input (Variables|PlayerInputs|Get3)
            (:True
              (bind _returnvalue_3 (UserInterface|CreateWidget "/Game/Blueprints/UI/Gameplay/InputUI/WBP_Input_3.WBP_Input_3_C" (Game|GetPlayerController 0)))
              (CallFunction|FAddWidgettoPlayerBox _returnvalue_3))
            (:False
              (Utilities|MCheckNumber Player%20Input (Variables|PlayerInputs|Get4)
                (:True
                  (bind _returnvalue_4 (UserInterface|CreateWidget "/Game/Blueprints/UI/Gameplay/InputUI/WBP_Input_4.WBP_Input_4_C" (Game|GetPlayerController 0)))
                  (CallFunction|FAddWidgettoPlayerBox _returnvalue_4))
                (:False
                  (Utilities|MCheckNumber Player%20Input (Variables|PlayerInputs|Get5)
                    (:True
                      (bind _returnvalue_5 (UserInterface|CreateWidget "/Game/Blueprints/UI/Gameplay/InputUI/WBP_Input_5.WBP_Input_5_C" (Game|GetPlayerController 0)))
                      (CallFunction|FAddWidgettoPlayerBox _returnvalue_5))
                    (:False
                      (Utilities|MCheckNumber Player%20Input (Variables|PlayerInputs|Get6)
                        (:True
                          (bind _returnvalue_6 (UserInterface|CreateWidget "/Game/Blueprints/UI/Gameplay/InputUI/WBP_Input_6.WBP_Input_6_C" (Game|GetPlayerController 0)))
                          (CallFunction|FAddWidgettoPlayerBox _returnvalue_6))
                        (:False
                          (Utilities|MCheckNumber Player%20Input (Variables|PlayerInputs|Get7)
                            (:True
                              (bind _returnvalue_7 (UserInterface|CreateWidget "/Game/Blueprints/UI/Gameplay/InputUI/WBP_Input_7.WBP_Input_7_C" (Game|GetPlayerController 0)))
                              (CallFunction|FAddWidgettoPlayerBox _returnvalue_7))
                            (:False
                              (Utilities|MCheckNumber Player%20Input (Variables|PlayerInputs|Get8)
                                (:True
                                  (bind _returnvalue_8 (UserInterface|CreateWidget "/Game/Blueprints/UI/Gameplay/InputUI/WBP_Input_8.WBP_Input_8_C" (Game|GetPlayerController 0)))
                                  (CallFunction|FAddWidgettoPlayerBox _returnvalue_8))
                                (:False
                                  (Utilities|MCheckNumber Player%20Input (Variables|PlayerInputs|Get9)
                                    (:True
                                      (bind _returnvalue_9 (UserInterface|CreateWidget "/Game/Blueprints/UI/Gameplay/InputUI/WBP_Input_9.WBP_Input_9_C" (Game|GetPlayerController 0)))
                                      (CallFunction|FAddWidgettoPlayerBox _returnvalue_9))))))))))))))))))))

(fn FClearPlayerInput&Box
  (Utilities|Array|Clear (Variables|TrickCombo|GetPlayerCombo))
  (Widget|Panel|ClearChildren (Variables|/Game/Blueprints/UI/Gameplay/WBP_ScreenInfo.WBP_ScreenInfo_C|GetHB_PlayerInputDisplay (Variables|Widget|GetScreenInfoWidgetRef))))

(fn FSetEnumOfRanomInt
  (params (RandomNum :type Integer))
  (if (== RandomNum 1)
    (Variables|ComboAnims|SetPlayerTrickAnimEnum "NewEnumerator1")
    (return)
    (elif (== RandomNum 2)
      (Variables|ComboAnims|SetPlayerTrickAnimEnum "NewEnumerator2")
      (return)
      (elif (== RandomNum 3)
        (Variables|ComboAnims|SetPlayerTrickAnimEnum "NewEnumerator3")
        (return)
        (elif (== RandomNum 4)
          (Variables|ComboAnims|SetPlayerTrickAnimEnum "NewEnumerator4")
          (return)
          (elif (== RandomNum 5)
            (Variables|ComboAnims|SetPlayerTrickAnimEnum "NewEnumerator5")
            (return)
            (elif (== RandomNum 6)
              (Variables|ComboAnims|SetPlayerTrickAnimEnum "NewEnumerator6")
              (return))))))))