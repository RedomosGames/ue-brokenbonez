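; Game instance for BrokenBonez that owns the BP_SaveGame data and exposes it through interface functions.
; On Init it synchronously loads the save slot, or creates a new save object in memory if none exists.
; Saving writes the whole object, optionally after updating player data, either sync or async.
; Only a completed async load calls the game-loaded notification.
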(event EventInit
  ;[1 1 0 0.5] Save Game Logic
  (CallFunction|IFLoadGameData false))

(event EventIFSavePlayer
  (params (PlayerSave :type S%20Player%20Save%20Structure) (Async? :type Boolean))
  ;[1 1 0 0.5] Save Game Logic
  (Variables|/Game/SaveGame/Blueprints/BP_SaveGame.BP_SaveGame_C|SetPlayerSave (Variables|Default|GetSavedData) PlayerSave)
  (CallFunction|IFSaveGameData Async?))

(event EventIFSaveGameData
  (params (Async? :type Boolean))
  ;[1 1 0 0.5] Save Game Logic
  ;;[1 1 0 0.5] Save Game
  (if Async?
    (|AsyncSaveGametoSlot (Variables|Default|GetSavedData) (Variables|Default|GetSlotName))
    (else
      (SaveGame|SaveGametoSlot (Variables|Default|GetSavedData) (Variables|Default|GetSlotName)))))

(event EventIFLoadGameData
  (params (Async? :type Boolean))
  ;[1 1 0 0.5] Save Game Logic
  ;;[1 1 0 0.5] Load Game
  (bind _returnvalue (SaveGame|DoesSaveGameExist (Variables|Default|GetSlotName)))
  (if _returnvalue
    (if Async?
      (bind _savegame (|AsyncLoadGamefromSlot (Variables|Default|GetSlotName))
        (:Completed
          (bind _asbp_save_game (Utilities|Casting|CastToBP_SaveGame _savegame))
          (Variables|Default|SetSavedData _asbp_save_game)
          (Default|CallOnGameLoaded)))
      (else
        (bind _returnvalue_2 (SaveGame|LoadGamefromSlot (Variables|Default|GetSlotName)))
        (bind _asbp_save_game_2 (Utilities|Casting|CastToBP_SaveGame _returnvalue_2))
        (Variables|Default|SetSavedData _asbp_save_game_2)))
    (else
      (bind _returnvalue_3 (SaveGame|CreateSaveGameObject "/Game/SaveGame/Blueprints/BP_SaveGame.BP_SaveGame_C"))
      (Variables|Default|SetSavedData _returnvalue_3))))

(fn IFGetGameData
  (return (Variables|Default|GetSavedData)))