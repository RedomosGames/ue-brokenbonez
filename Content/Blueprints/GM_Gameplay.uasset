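; GM_Gameplay is a gameplay Blueprint that runs the match countdown and signals game over when time runs out.
; BeginPlay waits briefly, then CE_StartGame starts a looping one-second timer bound to StartGame and stores its handle.
; Each tick decrements GameTimerLeft; at zero or below it calls OnGameOver and pauses the timer through the stored handle.
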(event Custom|CE_StartGame
  ;[1 0.783 0 0.5] CE_StartGame / Count Down Timer until game over
  (bind _returnvalue (Utilities|Time|SetTimerbyEvent (delegate Custom|StartGame) 1.0 true))
  (Variables|Default|SetGmeCountdownHandle _returnvalue))

(event Custom|StartGame
  ;[1 0.783 0 0.5] CE_StartGame / Count Down Timer until game over
  (bind _result (Math|Integer|DecrementInt (Variables|Default|GetGameTimerLeft))
    (:%20%20
      (if (<= _result 0)
        (Default|CallOnGameOver)
        (Utilities|Time|PauseTimerbyHandle (Variables|Default|GetGmeCountdownHandle))))))

(event EventBeginPlay
  ;[1 0.783 0 0.5] Begin Play
  (Utilities|FlowControl|Delay 1.0)
  (CallFunction|CEStartGame))

(fn ConstructionScript)